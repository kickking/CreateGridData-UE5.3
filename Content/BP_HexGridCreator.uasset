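; BP_HexGridCreator is a hex grid creator Blueprint that displays its status through an on-screen HUD.
; BeginPlay creates a WB_HUD widget, adds it to the viewport, calls the parent BeginPlay and starts a looping timer.
; The timer regularly passes the creator to the HUD's UpdateSubWidget if the HUD is valid.
; GetStateText turns the WorkFlowState enum into readable text by stripping its type prefix.
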(event Custom|UpdateHUD
  (bind _hud (Variables|Default|GetHUD)
    (:then
      (Default|UpdateSubWidget _hud self))
    (:else)))

(event EventBeginPlay
  (bind _returnvalue (UserInterface|CreateWidget "/Game/WB_HUD.WB_HUD_C"))
  (bind _output_get (Variables|Default|SetHUD _returnvalue))
  (UserInterface|Viewport|AddtoViewport _output_get 0)
  (|CallParentFunction)
  (Utilities|Time|SetTimerbyEvent (delegate Custom|UpdateHUD) 0.2 true))

(fn ConstructionScript)

(fn GetStateText
  (bind _workflowstate (Variables|Default|GetWorkFlowState))
  (bind _returnvalue (Utilities|Name|EnumtoName _workflowstate))
  (bind _returnvalue_2 (Utilities|String|ToString(Name) _returnvalue))
  (return (Utilities|Text|ToText(String) (Utilities|String|GetSubstring _returnvalue_2 (+ (Utilities|String|FindSubstring _returnvalue_2 "::") 2) (Utilities|String|Len _returnvalue_2)))))